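; BP_MainHUD is the game's HUD Blueprint, owning the player's main UI plus the victory and death screens.
; On BeginPlay it creates the main, victory and death widgets, adds them all to the viewport and keeps references.
; Its custom events forward calls to those widgets to update life and ammo bars, reveal the ammo bar on rifle pickup and show either end screen.
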(event `self.ReceiveBeginPlay`
  ;[1 1 1] creo la main ui (vida y ammo)
  (bind _returnvalue (`|CreateWidget` "/Game/FirstPerson/Blueprints/Widgets/WBP_MainUI.WBP_MainUI_C"))
  (bind _output_get (set `self.MainUIRef` _returnvalue))
  (`UserWidget.AddToViewport` _output_get 0)
  ;[1 1 1] creo el victory widget
  (bind _returnvalue_2 (`|CreateWidget` "/Game/FirstPerson/Blueprints/Widgets/WBP_Victory.WBP_Victory_C"))
  (bind _output_get_2 (set `self.VictoryUIRef` _returnvalue_2))
  (`UserWidget.AddToViewport` _output_get_2 0)
  ;[1 1 1] creo el death widget
  (bind _returnvalue_3 (`|CreateWidget` "/Game/FirstPerson/Blueprints/Widgets/WBP_Death.WBP_Death_C"))
  (bind _output_get_3 (set `self.DeathUIRef` _returnvalue_3))
  (`UserWidget.AddToViewport` _output_get_3 0))

(event `SetLifeBarMainUI`
  (params (currentLife :type "Float (double-precision)") (maxLife :type "Float (double-precision)"))
  (`/Game/FirstPerson/Blueprints/Widgets/WBP_MainUI.SetLifeBar` (`self.MainUIRef`) currentLife maxLife))

(event `ShowVictoryUI`
  (`/Game/FirstPerson/Blueprints/Widgets/WBP_Victory.ShowVictoryScreen` (`self.VictoryUIRef`)))

(event `ShowDeathUI`
  (`/Game/FirstPerson/Blueprints/Widgets/WBP_Death.ShowDeathScreen` (`self.DeathUIRef`)))

(event `SetAmmoBarMainUI`
  (params (currentAmmo :type Integer) (maxAmmo :type Integer))
  (`/Game/FirstPerson/Blueprints/Widgets/WBP_MainUI.SetAmmoBar` (`self.MainUIRef`) currentAmmo maxAmmo))

(event `OnGetRifleHUD`
  (`/Game/FirstPerson/Blueprints/Widgets/WBP_MainUI.ShowAmmoBar` (`self.MainUIRef`)))

(fn `UserConstructionScript`)